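; BP_PongBall is the Pong ball Blueprint, layering trail, respawn effect and sound feedback onto its parent class's behavior.
; It extends the parent's match-state handler to activate the trail effect when the match enters Waiting.
; On ball reset it calls the parent, deactivates the trail, then after a short delay triggers the respawn effect and a 2D spawn sound.
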(event `self.OnMatchStateChanged`
  (params (NewMatchState :type "EMatchState Enum" :default "Waiting"))
  (`parent.OnMatchStateChanged` NewMatchState)
  (if (`|EnumEquality` NewMatchState "Waiting")
    (`ActorComponent.Activate` (`self.NS_BallTrail`) false)))

(event `self.ResetBall`
  (`parent.ResetBall`)
  (`ActorComponent.Deactivate` (`self.NS_BallTrail`))
  (`KismetSystemLibrary.Delay` 1.25)
  (`ActorComponent.Activate` (`self.NS_BallRespawn`) false)
  (`GameplayStatics.PlaySound2D` (`self.BallSpawnSound`) 1.0 1.0 0.0 null null))

(fn `UserConstructionScript`)